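; BP_SpecOverlay manages a W_SpecOverlay spectator HUD in Mordhau team modes.
; After a delayed cosmetic-only start, a one-second timer checks the local player's team, using paired DoOnce gates to add the widget for team -1 and remove it otherwise.
; Adding it registers scale and enable console commands, unregistered on EndPlay.
; Both scale callbacks target element 0, and re-enabling does not immediately restore the overlay.
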(event Custom|CheckShowOverlay
  (if (== (Variables|/Script/Mordhau.MordhauPlayerState|GetTeam (.AsMordhau%20Player%20State (Utilities|Casting|CastToMordhauPlayerState (Variables|/Script/Engine.Controller|GetPlayerState (Game|GetPlayerController 0))))) -1)
    (Utilities|FlowControl|Sequence
      (:then_0
        (Utilities|FlowControl|DoOnce false :!label _label
          (:Completed
            (if (Variables|Default|GetEnabled)
              (CallFunction|AddOverlay)))))
      (:then_1
        (goto _label_2 Reset)))
    (else
      (Utilities|FlowControl|Sequence
        (:then_0
          (Utilities|FlowControl|DoOnce false :!label _label_2
            (:Completed
              (CallFunction|RemoveOverlay))))
        (:then_1
          (goto _label Reset))))))

(event EventBeginPlay
  (Networking|CanExecuteCosmeticEvents
    (:True
      (Utilities|FlowControl|Delay 3.0)
      (bind _asmordhau_game_state (Utilities|Casting|CastToMordhauGameState (Game|GetGameState)))
      (if (Variables|/Script/Mordhau.MordhauGameState|GetbIsTeamMode _asmordhau_game_state)
        (Utilities|Time|SetTimerbyEvent (delegate Custom|CheckShowOverlay) 1.0 true)))))

(event EventEndPlay
  (params (EndPlayReason :type EEndPlayReason%20Enum :default "Destroyed"))
  (bind _asbp_mordhau_player_controller (Utilities|Casting|CastToBP_MordhauPlayerController (Game|GetPlayerController 0)))
  (Class|MordhauPlayerController|UnregisterConsoleCommand _asbp_mordhau_player_controller "SpecOverlay.ScoreScale")
  (Class|MordhauPlayerController|UnregisterConsoleCommand _asbp_mordhau_player_controller "SpecOverlay.PlayerScale")
  (Class|MordhauPlayerController|UnregisterConsoleCommand _asbp_mordhau_player_controller "SpecOverlay.Enabled"))

(fn ConstructionScript)

(fn AddOverlay
  (bind _returnvalue (UserInterface|CreateWidget "/NeedyComp/SpecOverlay/W_SpecOverlay.W_SpecOverlay_C"))
  (bind _output_get (Variables|Default|SetOverlayRef _returnvalue))
  (UserInterface|Viewport|AddtoViewport _output_get -10)
  (bind _asbp_mordhau_player_controller (Utilities|Casting|CastToBP_MordhauPlayerController (Game|GetPlayerController 0)))
  (Class|MordhauPlayerController|RegisterConsoleCommand _asbp_mordhau_player_controller (Utilities|Struct|MakeMordhauConsoleCommand "SpecOverlay.ScoreScale" "Changes the scale of the UI. Default 1.0" (EventDispatchers|CreateEvent :!event BPSpecOverlayAutoGenFunc)))
  (Class|MordhauPlayerController|RegisterConsoleCommand _asbp_mordhau_player_controller (Utilities|Struct|MakeMordhauConsoleCommand "SpecOverlay.PlayerScale" "Changes the scale of the UI. Default 1.0" (EventDispatchers|CreateEvent :!event BPSpecOverlayAutoGenFunc1)))
  (Class|MordhauPlayerController|RegisterConsoleCommand _asbp_mordhau_player_controller (Utilities|Struct|MakeMordhauConsoleCommand "SpecOverlay.Enabled" "1 to show, 0 to hide" (EventDispatchers|CreateEvent :!event BPSpecOverlayAutoGenFunc2))))

(fn RemoveOverlay
  (bind _foundwidgets (Widget|GetAllWidgetsOfClass "/NeedyComp/SpecOverlay/W_SpecOverlay.W_SpecOverlay_C" false))
  (for _array_element _foundwidgets
    (Widget|RemovefromParent _array_element)))

(fn BPSpecOverlayAutoGenFunc
  (params (Params :type Array%20of%20Strings))
  (Default|SetScale (Variables|Default|GetOverlayRef) (Math|Conversions|ToFloat(Integer) (Utilities|Array|Get(acopy) Params))))

(fn BPSpecOverlayAutoGenFunc1
  (params (Params :type Array%20of%20Strings))
  (Default|SetScale (Variables|Default|GetOverlayRef) (Math|Conversions|ToFloat(Integer) (Utilities|Array|Get(acopy) Params))))

(fn BPSpecOverlayAutoGenFunc2
  (params (Params :type Array%20of%20Strings))
  (bind _output_get (Variables|Default|SetEnabled (Utilities|Select :Index (Math|Conversions|ToInteger(Byte) (Utilities|Array|Get(acopy) Params)) :Option%200 false :Option%201 true)))
  (if _output_get
    _
    (else
      (CallFunction|RemoveOverlay)))
  (return))