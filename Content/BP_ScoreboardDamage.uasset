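; BetterPUG mod actor for Mordhau team modes that adds admin match controls and a damage scoreboard.
; On authority it parses admin chat to move players to the other team or spectator, or toggle the team lock that Tick copies to the local controller.
; It also spawns a spectator overlay and, for team-HUD modes, swaps in a damage HUD.
; CheckDamage binds damage events, totalling in-progress enemy damage server-side and copying it to DmgRep.
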(event Custom|SRV%20Change%20Team
  (params (Player :type Mordhau%20Player%20State%20Object%20Reference) (Spec? :type Boolean))
  (bind _returnvalue (Class|MordhauPlayerState|GetLastPossessedMordhauCharacter Player))
  (if (Math|Boolean|Equal(Boolean) (Class|AdvancedCharacter|GetIsDead _returnvalue) false)
    (Game|Damage|ApplyDamage _returnvalue 999.0 0 0 "/Engine/EngineDamageTypes/DmgTypeBP_Environmental.DmgTypeBP_Environmental_C"))
  (Class|MordhauPlayerState|SetTeam Player (Math|Integer|SelectInt -1 (Math|Integer|SelectInt 1 0 (== (Variables|/Script/Mordhau.MordhauPlayerState|GetTeam Player) 0)) Spec?)))

(event Custom|CheckDamage
  (bind _returnvalue (Game|GetGameState))
  (bind _playerarray (Variables|/Script/Engine.GameStateBase|GetPlayerArray _returnvalue))
  (Variables|Default|SetPlayerStateOrderRep _playerarray)
  (for (_array_element _array_index) _playerarray
    (Utilities|Array|SetArrayElem (Variables|Default|GetDmgRep) _array_index (.Value (Utilities|Map|Find (Variables|Default|GetPlayerDamagesServerOnly) _array_element)) true)
    (bind _asmordhau_player_controller (Utilities|Casting|CastToMordhauPlayerController (Components|GetOwner _array_element)))
    (EventDispatchers|BindEventtoOnInstigatedAnyDamage _asmordhau_player_controller (delegate Custom|CustomEvent_0))))

(event Custom|CustomEvent_0
  (params (Damage :type Float%20%28single-precision%29) (DamageType :type Damage%20Type%20Object%20Reference) (DamagedActor :type Actor%20Object%20Reference) (DamageCauser :type Actor%20Object%20Reference))
  ;[1 1 1] On Damage Dealt
  (if (Utilities|Name|Equal(Name) (Variables|/Script/Engine.GameState|GetMatchState (.AsMordhau%20Game%20State (Utilities|Casting|CastToMordhauGameState (Game|GetGameState)))) "InProgress") ; Not in warmup?
    (bind _asmordhau_character (Utilities|Casting|CastToMordhauCharacter DamageCauser))
    (if (not (== (Variables|/Script/Mordhau.AdvancedCharacter|GetTeam (.AsMordhau%20Character (Utilities|Casting|CastToMordhauCharacter DamagedActor))) (Variables|/Script/Mordhau.AdvancedCharacter|GetTeam _asmordhau_character))) ; is team hit?
      (Utilities|Map|Add (Variables|Default|GetPlayerDamagesServerOnly) (Variables|/Script/Engine.Pawn|GetPlayerState _asmordhau_character) (Math|Float|SelectFloat (+ (.Value (Utilities|Map|Find (Variables|Default|GetPlayerDamagesServerOnly) (Variables|/Script/Engine.Pawn|GetPlayerState _asmordhau_character))) Damage) Damage (.ReturnValue (Utilities|Map|Find (Variables|Default|GetPlayerDamagesServerOnly) (Variables|/Script/Engine.Pawn|GetPlayerState _asmordhau_character))))))))

(event Custom|CustomEvent_2
  (params (Sender :type Actor%20Object%20Reference) (Msg :type String) (Type :type Name))
  (bind _asmordhau_player_controller (Utilities|Casting|CastToMordhauPlayerController Sender))
  (if (Class|MordhauPlayerController|IsAdmin _asmordhau_player_controller)
    (bind (_found _index _rights) (CallFunction|FindCommandsinString Msg))
    (if _found
      (switch int _index
        (:0
          (CallFunction|CommandMovePlayer (Utilities|Array|MakeArray _rights) false))
        (:1
          (CallFunction|CommandMovePlayer (Utilities|Array|MakeArray _rights) true))
        (:2
          (bind _output_get (Variables|Default|SetTeamSelectAllowed (not (Variables|Default|GetTeamSelectAllowed))))
          (CallFunction|MCMessage (Utilities|String|Append "TEAMS " (Utilities|String|SelectString "UNLOCKED" "LOCKED" _output_get)) (Utilities|Text|FormatText "Teams have been {a} by {name}." (Utilities|String|SelectString "UNLOCKED" "LOCKED" _output_get) (PlayerState|GetPlayerName (Variables|/Script/Engine.Controller|GetPlayerState _asmordhau_player_controller))) (Math|Color|SelectColor "(R=0.107439,G=0.687500,B=0.000000,A=1.000000)" "(R=1.000000,G=0.000000,B=0.040099,A=1.000000)" _output_get)))))))

(event Custom|MC%20Message
  (params (Name :type String) (Message :type Text) (NameColor :type Linear%20Color%20Structure :default "(R=0.000000,G=1.000000,B=0.853491,A=1.000000)"))
  (Utilities|FlowControl|Delay 0.2)
  (bind _asbp_mordhau_hud (Utilities|Casting|CastToBP_MordhauHUD (Class|MordhauUtilityLibrary|GetMordhauHUD)))
  (Default|AddEntry :self (Variables|/Game/Mordhau/Blueprints/BP_MordhauHUD.BP_MordhauHUD_C|GetChatBox _asbp_mordhau_hud) :Name Name :Message Message :NameColor NameColor :Prefix "BetterPUG"))

(event Custom|Load%20Message
  (if (Variables|Default|GetTeamSelectAllowed)
    (bind _asbp_mordhau_hud (Utilities|Casting|CastToBP_MordhauHUD (Class|MordhauUtilityLibrary|GetMordhauHUD)))
    (Default|AddEntry :self (Variables|/Game/Mordhau/Blueprints/BP_MordhauHUD.BP_MordhauHUD_C|GetChatBox _asbp_mordhau_hud) :Name "BetterPUG by swiift" :Message "BetterPUG has been loaded!" :NameColor "(R=0.000000,G=0.680716,B=0.937500,A=1.000000)")
    (else
      (bind _asbp_mordhau_hud_2 (Utilities|Casting|CastToBP_MordhauHUD (Class|MordhauUtilityLibrary|GetMordhauHUD)))
      (Default|AddEntry :self (Variables|/Game/Mordhau/Blueprints/BP_MordhauHUD.BP_MordhauHUD_C|GetChatBox _asbp_mordhau_hud_2) :Name "Teams locked" :Message "Teams are currently locked by an admin." :NameColor "(R=0.937500,G=0.058146,B=0.000000,A=1.000000)" :Prefix "BetterPUG"))))

(event EventBeginPlay
  (bind _asmordhau_game_state (Utilities|Casting|CastToMordhauGameState (Game|GetGameState)))
  (if (Variables|/Script/Mordhau.MordhauGameState|GetbIsTeamMode _asmordhau_game_state)
    (Networking|SwitchHasAuthority
      (:Authority
        (Utilities|FlowControl|Sequence
          (:then_0
            (Game|SpawnActorfromClass "/NeedyComp/SpecOverlay/BP_SpecOverlay.BP_SpecOverlay_C" (Math|Transform|MakeTransform "0, 0, 0") "Undefined" 0 0)
            (bind _asmordhau_game_mode (Utilities|Casting|CastToMordhauGameMode (Game|GetGameMode)))
            (EventDispatchers|BindEventtoOnMessageBroadcasted _asmordhau_game_mode (delegate Custom|CustomEvent_2)))
          (:then_1
            ;[1 1 1] skm only
            (bind _asmordhau_game_mode_2 (Utilities|Casting|CastToMordhauGameMode (Game|GetGameMode)))
            (Utilities|Casting|CastToBP_MordhauTeamHUDClass (Variables|/Script/Engine.GameModeBase|GetHUDClass _asmordhau_game_mode_2))
            (Variables|/Script/Mordhau.MordhauGameMode|SetTeamKillScoreChange _asmordhau_game_mode_2 0.0)
            (Variables|/Script/Engine.GameModeBase|SetHUDClass _asmordhau_game_mode_2 "/NeedyComp/HUD_SKM_Dmg.HUD_SKM_Dmg_C")
            (Utilities|Time|SetTimerbyEvent (EventDispatchers|CreateEvent :!event Custom|CheckDamage) 1.0 true)))))))

(event EventTick
  (params (DeltaSeconds :type Float%20%28single-precision%29))
  (bind _asbp_mordhau_player_controller (Utilities|Casting|CastToBP_MordhauPlayerController (Game|GetPlayerController 0)))
  (Variables|/Game/Mordhau/Blueprints/BP_MordhauPlayerController.BP_MordhauPlayerController_C|SetbIsTeamSelectAvailable _asbp_mordhau_player_controller (Variables|Default|GetTeamSelectAllowed)))

(fn ConstructionScript)

(fn CommandMovePlayer
  (params (Params :type Array%20of%20Strings) (Spec? :type Boolean))
  (bind _output (Utilities|Array|Get(acopy) Params))
  (Utilities|CheckAdmin
    (:true
      (Development|PrintString _output)
      (bind _returnvalue (Class|MordhauUtilityLibrary|FindPlayerState _output))
      (Utilities|IsValid _returnvalue
        (:Is%20Valid
          (bind _asbp_mordhau_player_state (Utilities|Casting|CastToBP_MordhauPlayerState _returnvalue)
            (:then
              (CallFunction|SRVChangeTeam _asbp_mordhau_player_state Spec?))
            (:CastFailed
              (Development|PrintString "Failed to find player" :!label _label)
              (Class|MordhauUtilityLibrary|PrinttoConsoleandLog "Failed to find player" false))))
        (:Is%20Not%20Valid
          (bind (_character _found_) (CallFunction|FindPlayer _output))
          (if _found_
            (bind _asbp_mordhau_player_state_2 (Utilities|Casting|CastToBP_MordhauPlayerState _character)
              (:then
                (CallFunction|SRVChangeTeam _asbp_mordhau_player_state_2 Spec?))
              (:CastFailed
                (goto _label)))
            (else
              (goto _label)))))
      (return))))

(fn FindPlayer
  (params (name :type String))
  (bind _matches (LocalVariables|GetMatches))
  (bind _output (Utilities|Array|Get(acopy) _matches))
  (for _array_element (Variables|/Script/Engine.GameStateBase|GetPlayerArray (Game|GetGameState))
    (if (Utilities|String|Contains (PlayerState|GetPlayerName _array_element) name)
      (Utilities|Array|Add (LocalVariables|GetMatches) _array_element)))
  (if (> (Utilities|Array|Length (LocalVariables|GetMatches)) 1)
    (for _array_element_2 (LocalVariables|GetMatches)
      (if (Utilities|Enum|Equal(Enum) (PlayerState|GetPlayerName _array_element_2) name)
        (return _array_element_2 true)))
    (else
      (return _output (Utilities|IsValid _output)))))

(fn SetPaused
  (bind _output_get (Variables|Default|SetPaused (not (Variables|Default|GetPaused))))
  (bind _asbp_mordhau_game_state (Utilities|Casting|CastToBP_MordhauGameState (Game|GetGameState)))
  (Variables|/Script/Mordhau.MordhauGameState|SetWarmupEnd _asbp_mordhau_game_state (Math|Float|SelectFloat 9999999.0 (+ (GameState|GetServerWorldTimeSeconds _asbp_mordhau_game_state) 1.0) _output_get)))

(fn FindCommandsinString
  (params (SearchIn :type String))
  (LocalVariables|SetReturnedCommand -1)
  (for (_array_element _array_index) (Variables|Default|GetCommands%20to%20Parse)
    (if (Utilities|String|Contains SearchIn _array_element)
      (LocalVariables|SetReturnedCommand _array_index)))
  (return (not (== (LocalVariables|GetReturnedCommand) -1)) (LocalVariables|GetReturnedCommand) (.RightS (Utilities|String|Split SearchIn (Utilities|String|Append (Utilities|Array|Get(acopy) (Variables|Default|GetCommands%20to%20Parse) (LocalVariables|GetReturnedCommand)) " ")))))